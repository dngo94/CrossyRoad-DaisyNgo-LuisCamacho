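; BP_DRoadLeft is a road actor that keeps left-bound traffic looping, with a police car and a taxi.
; On BeginPlay it spawns BP_policeLeft and BP_taxiLeft at two spawn point components, both with the same fixed yaw.
; When each car type overlaps its trigger zone, a replacement spawns at that type's spawn point and the arriving car is destroyed, so each lane recycles one car.
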(event `self.ReceiveBeginPlay`
  (`self.SpawnCar` (`SceneComponent.K2_GetComponentLocation` (`self.spawnpoint1`)))
  (`self.spawnCar2` (`SceneComponent.K2_GetComponentLocation` (`self.spawnpoint2`))))

(event `self.triggerzone.OnComponentBeginOverlap`
  (params (OverlappedComponent :type "PrimitiveComponent Object Reference") (OtherActor :type "Actor Object Reference") (OtherComp :type "PrimitiveComponent Object Reference") (OtherBodyIndex :type Integer) (bFromSweep :type Boolean) (SweepResult :type "HitResult Structure (by ref)"))
  (bind _asbp_police_left (cast `/Game/blueprint/BP_policeLeft` OtherActor))
  (`self.spawnCarsAtSpawnPoint ` (`self.spawnpoint1`))
  (`self.K2_DestroyActor` _asbp_police_left))

(event `self.triggerzone2.OnComponentBeginOverlap`
  (params (OverlappedComponent :type "PrimitiveComponent Object Reference") (OtherActor :type "Actor Object Reference") (OtherComp :type "PrimitiveComponent Object Reference") (OtherBodyIndex :type Integer) (bFromSweep :type Boolean) (SweepResult :type "HitResult Structure (by ref)"))
  (bind _asbp_taxi_left (cast `/Game/blueprint/BP_taxiLeft` OtherActor))
  (`self.spawnCarsAtSpawnPoint2` (`self.spawnpoint2`))
  (`self.K2_DestroyActor` _asbp_taxi_left))

(fn `SpawnCar`
  (params (transform :type "Vector Structure") (NewParam :type Boolean))
  (`|SpawnActorFromClass` "/Game/blueprint/BP_policeLeft.BP_policeLeft_C" (`KismetMathLibrary.MakeTransform` transform (struct :`Yaw` 270.0)) "Undefined" "OverrideRootScale" null null))

(fn `spawnCar2`
  (params (`Spawn Transform Location` :type "Vector Structure") (NewParam :type Boolean))
  (`|SpawnActorFromClass` "/Game/blueprint/BP_taxiLeft.BP_taxiLeft_C" (`KismetMathLibrary.MakeTransform` `Spawn Transform Location` (struct :`Yaw` 270.0)) "Undefined" "OverrideRootScale" null null))

(fn `spawnCarsAtSpawnPoint `
  (params (spawnpoint1 :type "SceneComponent Object Reference"))
  (`self.SpawnCar` (`SceneComponent.K2_GetComponentLocation` spawnpoint1)))

(fn `spawnCarsAtSpawnPoint2`
  (params (spawnpoint2 :type "SceneComponent Object Reference"))
  (`self.spawnCar2` (`SceneComponent.K2_GetComponentLocation` spawnpoint2)))

(fn `UserConstructionScript`)