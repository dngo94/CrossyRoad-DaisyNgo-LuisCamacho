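; BP_SRoad is a road actor that keeps a car recycling along it.
; On BeginPlay it spawns a BP_Car at the location of Spawnpoint1 with a fixed rotation.
; When a BP_Car begins overlapping Triggerzone1, it spawns a replacement at the same spawn point and destroys the arriving car.
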(event `self.ReceiveBeginPlay`
  (`self.spawnCar1` (`SceneComponent.K2_GetComponentLocation` (`self.Spawnpoint1`))))

(event `self.Triggerzone1.OnComponentBeginOverlap`
  (params (OverlappedComponent :type "PrimitiveComponent Object Reference") (OtherActor :type "Actor Object Reference") (OtherComp :type "PrimitiveComponent Object Reference") (OtherBodyIndex :type Integer) (bFromSweep :type Boolean) (SweepResult :type "HitResult Structure (by ref)"))
  (bind _asbp_car (cast `/Game/blueprint/BP_Car` OtherActor))
  (`self.SpawnCarAtSpawnPoint1` (`self.Spawnpoint1`))
  (`self.K2_DestroyActor` _asbp_car))

(fn `spawnCar1`
  (params (`Spawn Transform Location` :type "Vector Structure"))
  (`|SpawnActorFromClass` "/Game/blueprint/BP_Car.BP_Car_C" (`KismetMathLibrary.MakeTransform` `Spawn Transform Location` (struct :`Yaw` 90.0)) "Undefined" "OverrideRootScale" null null))

(fn `SpawnCarAtSpawnPoint1`
  (params (spawnpoint1 :type "SceneComponent Object Reference"))
  (`self.spawnCar1` (`SceneComponent.K2_GetComponentLocation` spawnpoint1)))

(fn `UserConstructionScript`)