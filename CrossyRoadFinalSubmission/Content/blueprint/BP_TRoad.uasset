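; BP_TRoad is a road actor that keeps three kinds of vehicle traffic running: a truck, a car and a police vehicle.
; On BeginPlay it spawns one of each at its own spawn point, all with the same fixed rotation.
; When a vehicle of the matching class enters its trigger zone, the road spawns a replacement at that lane's spawn point and destroys the arriving one, forming an endless loop.
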(event `self.ReceiveBeginPlay`
  (`self.SpawnCar1` (`SceneComponent.K2_GetComponentLocation` (`self.SpawnPoint1`)))
  (`self.SpawnCar2` (`SceneComponent.K2_GetComponentLocation` (`self.SpawnPoint2`)))
  (`self.SpawnCar3` (`SceneComponent.K2_GetComponentLocation` (`self.SpawnPoint3`))))

(event `self.TriggerZone1.OnComponentBeginOverlap`
  (params (OverlappedComponent :type "PrimitiveComponent Object Reference") (OtherActor :type "Actor Object Reference") (OtherComp :type "PrimitiveComponent Object Reference") (OtherBodyIndex :type Integer) (bFromSweep :type Boolean) (SweepResult :type "HitResult Structure (by ref)"))
  (bind _asbp_truck (cast `/Game/blueprint/BP_TruckRight` OtherActor))
  (`self.SpawnCarAtSpawnPoint1` (`self.SpawnPoint1`))
  (`self.K2_DestroyActor` _asbp_truck))

(event `self.TriggerZone2.OnComponentBeginOverlap`
  (params (OverlappedComponent :type "PrimitiveComponent Object Reference") (OtherActor :type "Actor Object Reference") (OtherComp :type "PrimitiveComponent Object Reference") (OtherBodyIndex :type Integer) (bFromSweep :type Boolean) (SweepResult :type "HitResult Structure (by ref)"))
  (bind _asbp_car (cast `/Game/blueprint/BP_Car` OtherActor))
  (`self.SpawnCarAtSpawnPoint2` (`self.SpawnPoint2`))
  (`self.K2_DestroyActor` _asbp_car))

(event `self.TriggerZone3.OnComponentBeginOverlap`
  (params (OverlappedComponent :type "PrimitiveComponent Object Reference") (OtherActor :type "Actor Object Reference") (OtherComp :type "PrimitiveComponent Object Reference") (OtherBodyIndex :type Integer) (bFromSweep :type Boolean) (SweepResult :type "HitResult Structure (by ref)"))
  (bind _asbp_police_left (cast `/Game/blueprint/BP_policeRight` OtherActor))
  (`self.SpawnCarAtSpawnPoint3` (`self.SpawnPoint3`))
  (`self.K2_DestroyActor` _asbp_police_left))

(fn `SpawnCar1`
  (params (`Spawn Transform Location` :type "Vector Structure"))
  (`|SpawnActorFromClass` "/Game/blueprint/BP_TruckRight.BP_TruckRight_C" (`KismetMathLibrary.MakeTransform` `Spawn Transform Location` (struct :`Yaw` 90.0)) "Undefined" "OverrideRootScale" null null))

(fn `SpawnCar2`
  (params (`Spawn Transform Location` :type "Vector Structure"))
  (`|SpawnActorFromClass` "/Game/blueprint/BP_Car.BP_Car_C" (`KismetMathLibrary.MakeTransform` `Spawn Transform Location` (struct :`Yaw` 90.0)) "Undefined" "OverrideRootScale" null null))

(fn `SpawnCar3`
  (params (`Spawn Transform Location` :type "Vector Structure"))
  (`|SpawnActorFromClass` "/Game/blueprint/BP_policeRight.BP_policeRight_C" (`KismetMathLibrary.MakeTransform` `Spawn Transform Location` (struct :`Yaw` 90.0)) "Undefined" "OverrideRootScale" null null))

(fn `SpawnCarAtSpawnPoint1`
  (params (SpawnPoint1 :type "SceneComponent Object Reference"))
  (`self.SpawnCar1` (`SceneComponent.K2_GetComponentLocation` SpawnPoint1)))

(fn `SpawnCarAtSpawnPoint2`
  (params (SpawnPoint2 :type "SceneComponent Object Reference"))
  (`self.SpawnCar2` (`SceneComponent.K2_GetComponentLocation` SpawnPoint2)))

(fn `SpawnCarAtSpawnPoint3`
  (params (SpawnPoint3 :type "SceneComponent Object Reference"))
  (`self.SpawnCar3` (`SceneComponent.K2_GetComponentLocation` SpawnPoint3)))

(fn `UserConstructionScript`)