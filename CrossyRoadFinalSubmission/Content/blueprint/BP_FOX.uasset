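; BP_FOX is a player-controlled fox pawn that moves on input and dies, visually squashed, when its mesh overlaps something.
; Axis inputs scale by MaxSpeed into movement input, with MoveForward using the right vector and MoveRight the forward vector.
; Tick applies the consumed input as an unswept local offset until Dead is set.
; Pressing D turns the actor 90 degrees in yaw, gated by a DoOnce that resets on release.
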(event `InputAxis|MoveForward`
  (params (AxisValue :type "Float (single-precision)"))
  (`self.AddMovementInput` (`self.GetActorRightVector`) (* AxisValue (`self.MaxSpeed`))))

(event `InputAxis|MoveRight`
  (params (AxisValue :type "Float (single-precision)"))
  (`self.AddMovementInput` (`self.GetActorForwardVector`) (* AxisValue (`self.MaxSpeed`))))

(event `self.ReceiveTick`
  (params (DeltaSeconds :type "Float (single-precision)"))
  (if (not (`self.dead`))
    (bind _returnvalue (`self.ConsumeMovementInputVector`))
    (`self.K2_AddActorLocalOffset` _returnvalue)))

(event `self.StaticMesh.OnComponentBeginOverlap`
  (params (OverlappedComponent :type "PrimitiveComponent Object Reference") (OtherActor :type "Actor Object Reference") (OtherComp :type "PrimitiveComponent Object Reference") (OtherBodyIndex :type Integer) (bFromSweep :type Boolean) (SweepResult :type "HitResult Structure (by ref)"))
  (`SceneComponent.SetRelativeScale3D` (`self.StaticMesh`) (5.0 0.1 0.4))
  (set `self.dead` true))

(event `Key|D`
  (params (Key :type "Key Structure"))
  (bind (_returnvalue_roll _returnvalue_pitch _returnvalue_yaw) (`KismetMathLibrary.BreakRotator` (`self.K2_GetActorRotation`)))
  (:`Pressed`
    (`/Engine/EditorBlueprintResources/StandardMacros.DoOnce` false :!label _label
      (:`Completed`
        (`KismetSystemLibrary.PrintString` "d_pressed")
        (`self.K2_SetActorRotation` (`KismetMathLibrary.MakeRotator` 0.0 0.0 (+ _returnvalue_yaw 90.0))))))
  (:`Released`
    (goto _label :!via `Reset`)))

(fn `UserConstructionScript`)