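; BP_TrackLeft is a track actor that keeps a left-side train running by respawning it.
; On BeginPlay it spawns a BP_TrainLeft at SpawnPoint1 with a fixed rotation.
; When a BP_TrainLeft begins overlapping TriggerZone1, it spawns a replacement at SpawnPoint1 and destroys the arriving train, creating an endless loop.
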(event `self.ReceiveBeginPlay`
  (`self.SpawnTrain` (`SceneComponent.K2_GetComponentLocation` (`self.SpawnPoint1`))))

(event `self.TriggerZone1.OnComponentBeginOverlap`
  (params (OverlappedComponent :type "PrimitiveComponent Object Reference") (OtherActor :type "Actor Object Reference") (OtherComp :type "PrimitiveComponent Object Reference") (OtherBodyIndex :type Integer) (bFromSweep :type Boolean) (SweepResult :type "HitResult Structure (by ref)"))
  (bind _asbp_train_left (cast `/Game/blueprint/BP_TrainLeft` OtherActor))
  (`self.SpawnTrainAtSpawnPoint` (`self.SpawnPoint1`))
  (`self.K2_DestroyActor` _asbp_train_left))

(fn `SpawnTrain`
  (params (`Spawn Tranform` :type "Vector Structure"))
  (`|SpawnActorFromClass` "/Game/blueprint/BP_TrainLeft.BP_TrainLeft_C" (`KismetMathLibrary.MakeTransform` `Spawn Tranform` (struct :`Yaw` 90.0)) "Undefined" "OverrideRootScale" null null))

(fn `SpawnTrainAtSpawnPoint`
  (params (SpawnPoint1 :type "SceneComponent Object Reference"))
  (`self.SpawnTrain` (`SceneComponent.K2_GetComponentLocation` SpawnPoint1)))

(fn `UserConstructionScript`)